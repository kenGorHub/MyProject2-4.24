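; Test guard character Blueprint that performs a melee attack through a MeleeAttack event.
; The event plays a primary attack montage, and each notify begin fires a short sphere trace forward from the right-hand socket on the Camera channel, with persistent debug drawing.
; The hit actor goes to ReportDamageEvent with the guard as instigator, which reports damage to AI perception; no ApplyDamage call is made.
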(event `/Game/ThirdPersonBP/Blueprints/interface/Combat_interface.MeleeAttack`
  (bind _returnvalue (`SceneComponent.GetSocketLocation` (`self.Mesh`) "hand_rSocket"))
  (`|PlayMontage` (`self.Mesh`) "/Game/ThirdPersonBP/animation/combat/Attack_PrimaryA_Montage.Attack_PrimaryA_Montage"
    (:`OnNotifyBegin`
      (bind _outhit (`KismetSystemLibrary.SphereTraceSingle` :`Start` _returnvalue :`End` (+ _returnvalue (* (`KismetMathLibrary.GetForwardVector` (`self.K2_GetActorRotation`)) 50.0)) :`Radius` 40.0 :`TraceChannel` "TraceTypeQuery2" :`DrawDebugType` "Persistent"))
      (`AISense_Damage.ReportDamageEvent` (`.HitActor` (`GameplayStatics.BreakHitResult` _outhit)) self 10.0 (`.TraceStart` (`GameplayStatics.BreakHitResult` _outhit))))))

(fn `UserConstructionScript`)