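; Boss AI character with a montage-driven melee attack and a one-shot leap toward its target.
; MeleeAttack sphere-traces from the right hand on montage notify, reporting the hit actor to the AI damage sense rather than applying damage.
; While IsOneTime is set, Movement faces Target, launches the boss along the offset with an upward arc, then clears the flag.
; An AddMovementInput node is left unconnected.
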(event `/Game/ThirdPersonBP/Blueprints/interface/Combat_interface.MeleeAttack`
  (bind _returnvalue (`SceneComponent.GetSocketLocation` (`self.Mesh`) "hand_r"))
  (`|PlayMontage` (`self.Mesh`) "/Game/ThirdPersonBP/animation/combat/SK_Mannequin/Attack_PrimaryA_Montage.Attack_PrimaryA_Montage"
    (:`OnNotifyBegin`
      (bind _outhit (`KismetSystemLibrary.SphereTraceSingle` :`Start` _returnvalue :`End` (+ _returnvalue (* (`KismetMathLibrary.GetForwardVector` (`self.K2_GetActorRotation`)) 50.0)) :`Radius` 40.0 :`TraceChannel` "TraceTypeQuery2" :`DrawDebugType` "ForOneFrame"))
      (`AISense_Damage.ReportDamageEvent` (`.HitActor` (`GameplayStatics.BreakHitResult` _outhit)) self 10.0 (`.TraceStart` (`GameplayStatics.BreakHitResult` _outhit))))))

(fn `Movement`
  (bind (_returnvalue_x _returnvalue_y) (`KismetMathLibrary.BreakVector` (- (`self.K2_GetActorLocation` (`self.target`)) (`self.K2_GetActorLocation` self))))
  (if (`self.isOneTime?`)
    (`self.K2_SetActorRotation` (`KismetMathLibrary.FindLookAtRotation` (`self.K2_GetActorLocation` self) (`self.K2_GetActorLocation` (`self.target`))))
    (`self.LaunchCharacter` (`KismetMathLibrary.MakeVector` _returnvalue_x _returnvalue_y 600.0) true true)
    (set `self.isOneTime?` false))
  (return))

(fn `UserConstructionScript`)